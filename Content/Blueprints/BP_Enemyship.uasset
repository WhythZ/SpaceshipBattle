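; BP_Enemyship is an enemy ship actor that gives itself a random color scheme and plays a scale animation for its spawn.
; The SetRandomColor event creates a dynamic instance of M_Base_Ship, independently picks body and wing colors from two four-color palettes, and applies it to the mesh.
; The same event then plays SpawnScalingTimeline to drive the actor's uniform scale.
; Nothing in this Blueprint calls the event.
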(event EventBeginPlay)

(event Collision|EventActorBeginOverlap
  (params (OtherActor :type Actor%20Object%20Reference)))

(event EventTick
  (params (DeltaSeconds :type Float%20%28single-precision%29)))

(event EventSetRandomColor
  (Variables|Default|SetrandomColorBody (Math|Random|RandomIntegerinRange 0 3))
  (Variables|Default|SetrandomColorWing (Math|Random|RandomIntegerinRange 0 3))
  (bind _returnvalue (Rendering|Material|CreateDynamicMaterialInstance "/Game/Assets/Materials/M_Base_Ship.M_Base_Ship" "None" "None" :!class /Script/Engine.KismetMaterialLibrary))
  (Rendering|Material|SetVectorParameterValue _returnvalue "Color1" (Utilities|Select :Index (Variables|Default|GetrandomColorBody) :Option%200 "(R=0.911372,G=0.000000,B=1.000000,A=1.000000)" :Option%201 "(R=0.123003,G=1.000000,B=0.000000,A=1.000000)" :Option%202 "(R=0.000000,G=0.483937,B=1.000000,A=1.000000)" :Option%203 "(R=1.000000,G=0.000000,B=0.039560,A=1.000000)") :!class /Script/Engine.MaterialInstanceDynamic)
  (Rendering|Material|SetVectorParameterValue _returnvalue "Color2" (Utilities|Select :Index (Variables|Default|GetrandomColorWing) :Option%200 "(R=0.955130,G=0.319834,B=1.000000,A=1.000000)" :Option%201 "(R=0.331360,G=0.756944,B=0.288845,A=1.000000)" :Option%202 "(R=0.499952,G=0.920049,B=1.000000,A=1.000000)" :Option%203 "(R=0.906250,G=0.264323,B=0.264323,A=1.000000)") :!class /Script/Engine.MaterialInstanceDynamic)
  (Rendering|Material|SetMaterial (Variables|Default|GetenemyshipStaticMesh) 0 _returnvalue)
  (bind _shipscaling (Timeline|SpawnScalingTimeline Play)
    (:Update
      (Transformation|SetActorScale3D (Math|Conversions|ToVector(Float) _shipscaling)))))

(fn ConstructionScript)